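; BP_JumpPadVar1 is a jump pad that launches the third-person character upward when it enters the pad's Box trigger.
; After a short delay, it applies a vertical impulse through the CharacterMovement component, scaled by the magnitude of the character's last update velocity, so faster entries launch higher.
; A leftover AddImpulse node based on the root component's velocity is never executed.
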(event OnComponentBeginOverlap(Box)
  (params (OverlappedComponent :type Primitive%20Component%20Object%20Reference) (OtherActor :type Actor%20Object%20Reference) (OtherComp :type Primitive%20Component%20Object%20Reference) (OtherBodyIndex :type Integer) (bFromSweep :type Boolean) (SweepResult :type Hit%20Result%20Structure%20%28by%20ref%29))
  (bind _asbp_third_person_character (Utilities|Casting|CastToBP_ThirdPersonCharacter OtherActor))
  (Utilities|FlowControl|Delay 0.1)
  (Physics|AddImpulse (Variables|/Script/Engine.Character|GetCharacterMovement _asbp_third_person_character) (Math|Vector|MakeVector 0.0 0.0 (* (Math|Vector|VectorLength (Pawn|Components|CharacterMovement|GetLastUpdateVelocity (Variables|/Script/Engine.Character|GetCharacterMovement _asbp_third_person_character))) 3.5e+02)) false))

(fn ConstructionScript)