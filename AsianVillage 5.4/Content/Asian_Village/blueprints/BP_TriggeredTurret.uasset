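; BP_TriggeredTurret is a turret actor that fires BP_BulletFlat projectiles while its trigger volume is active.
; Begin and end overlap on the trigger volume switch actor tick on and off, with no filter on the overlapping actor.
; Each tick spawns a bullet at the spawn point's transform with a configurable scale and lifespan, so fire rate follows frame or tick rate.
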(event OnComponentBeginOverlap(TriggerVolume)
  (params (OverlappedComponent :type Primitive%20Component%20Object%20Reference) (OtherActor :type Actor%20Object%20Reference) (OtherComp :type Primitive%20Component%20Object%20Reference) (OtherBodyIndex :type Integer) (bFromSweep :type Boolean) (SweepResult :type Hit%20Result%20Structure%20%28by%20ref%29))
  (Actor|Tick|SetActorTickEnabled true))

(event OnComponentEndOverlap(TriggerVolume)
  (params (OverlappedComponent :type Primitive%20Component%20Object%20Reference) (OtherActor :type Actor%20Object%20Reference) (OtherComp :type Primitive%20Component%20Object%20Reference) (OtherBodyIndex :type Integer))
  (Actor|Tick|SetActorTickEnabled false))

(event EventTick
  (params (DeltaSeconds :type Float%20%28single-precision%29))
  (bind _spawnpoint (Variables|Default|GetSpawnPoint))
  (bind _returnvalue (Game|SpawnActorfromClass "/Game/Asian_Village/blueprints/BP_BulletFlat.BP_BulletFlat_C" (Math|Transform|MakeTransform (Transformation|GetWorldLocation _spawnpoint) (Transformation|GetWorldRotation _spawnpoint) (Math|Conversions|ToVector(Float) (Variables|Default|GetProjectileScale))) "Undefined" "MultiplyWithRoot" 0 0))
  (Actor|SetLifeSpan _returnvalue (Variables|Default|GetIn%20Lifespan)))

(fn ConstructionScript)