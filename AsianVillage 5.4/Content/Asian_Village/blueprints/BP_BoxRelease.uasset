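; BP_BoxRelease is a box with a door that swings open and a mover that travels along preset points.
; The construction script feeds Location01, Location02 and further relative control points, plus a Duration, into an InterpToMovement component.
; The ActivateMovement event plays a Rotate timeline that drives the yaw of BoxDoor's relative rotation.
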(event Custom|ActivateMovement
  (bind _rotate (Timeline|Rotate Play)
    (:Update
      (Transformation|SetRelativeRotation (Variables|Default|GetBoxDoor) (Math|Rotator|MakeRotator 0.0 0.0 _rotate) false false))))

(fn ConstructionScript
  (bind _interptomovement (Variables|Default|GetInterpToMovement))
  (Variables|/Script/Engine.InterpToMovementComponent|SetControlPoints _interptomovement (Utilities|Array|MakeArray (Utilities|Struct|MakeInterpControlPoint (Variables|Default|GetLocation01) true) (Utilities|Struct|MakeInterpControlPoint (Variables|Default|GetLocation02) true) ""))
  (Variables|/Script/Engine.InterpToMovementComponent|SetDuration _interptomovement (Variables|Default|GetDuration)))